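; BP_Key is a pickup that stays hidden and non-collidable until no BP_MovingTarget actors remain in the level.
; Tick polls for targets, taking the count from the index returned by an array Add, and toggles mesh visibility and collision.
; A DoOnce plays an explosion effect and sound on reveal.
; When the first-person character overlaps the revealed key's sphere, it sets HasKey, plays the sound and destroys itself.
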(event `self.ReceiveBeginPlay`
  (bind _asbp_first_person_character (cast `/Game/FirstPerson/Blueprints/BP_FirstPersonCharacter` (`GameplayStatics.GetPlayerCharacter` 0)))
  (set `self.As BP First Person Character` _asbp_first_person_character))

(event `self.Sphere_Collider.OnComponentBeginOverlap`
  (params (OverlappedComponent :type "PrimitiveComponent Object Reference") (OtherActor :type "Actor Object Reference") (OtherComp :type "PrimitiveComponent Object Reference") (OtherBodyIndex :type Integer) (bFromSweep :type Boolean) (SweepResult :type "HitResult Structure (by ref)"))
  ;[0.4244 1 0.3612] Collect Key
  (if (and (== OtherActor (`self.As BP First Person Character`)) (`self.AllTargetsDestroyed`))
    (set `/Game/FirstPerson/Blueprints/BP_FirstPersonCharacter.HasKey` true (`self.As BP First Person Character`))
    (`GameplayStatics.PlaySoundAtLocation` "/Game/StarterContent/Audio/Explosion01.Explosion01" (`self.K2_GetActorLocation`) (struct) 1.0 1.0 0.0 null null null null)
    (`self.K2_DestroyActor`)))

(event `self.ReceiveTick`
  (params (DeltaSeconds :type "Float (single-precision)"))
  (bind _returnvalue (`self.K2_GetActorLocation`))
  ;[1 0.7481 0.2744] Key Visibility
  (bind _outactors (`GameplayStatics.GetAllActorsOfClass` "/Game/Microgames/Blueprints/BP_MovingTarget.BP_MovingTarget_C"))
  (bind _returnvalue_2 (`KismetArrayLibrary.Array_Add` _outactors))
  (bind _output_get (set `self.AllTargetsDestroyed` (<= _returnvalue_2 0)))
  (`SceneComponent.SetVisibility` (`self.SM_Key`) _output_get true)
  (`self.SetActorEnableCollision` _output_get)
  ;[0.28 0.8291 1] Spawn Sound
  (if (`self.AllTargetsDestroyed`)
    (`/Engine/EditorBlueprintResources/StandardMacros.DoOnce` false
      (:`Completed`
        (`GameplayStatics.SpawnEmitterAtLocation` "/Game/StarterContent/Particles/P_Explosion.P_Explosion" _returnvalue)
        (`GameplayStatics.PlaySoundAtLocation` "/Game/StarterContent/Audio/Explosion01.Explosion01" _returnvalue (struct) 1.0 1.0 0.0 null null null null)))))

(fn `UserConstructionScript`)